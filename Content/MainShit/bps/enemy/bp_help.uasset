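; Enemy pawn that chases the first-person player and plays a sound cue when play begins.
; PawnSensing triggers AI movement toward the spotted player, while a self-calling event with a tiny Delay keeps interpolating its yaw to face them.
; A projectile hit or bp_meanbox overlap plays a death sound and destroys it after a brief delay.
; The FacePlayer function is empty.
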(event `self.ReceiveBeginPlay`
  (`AudioComponent.Play` (`self.fuck_you_cue`) 0.0)
  (bind _asfirst_person_character (cast `/Game/FirstPersonBP/Blueprints/FirstPersonCharacter` (`GameplayStatics.GetPlayerCharacter` 0)))
  (set `self.player_ref` _asfirst_person_character)
  (`self.my ass`))

(event `self.PawnSensing.OnSeePawn`
  (params (Pawn :type "Pawn Object Reference"))
  ;[1 1 1] ai shit
  (bind _asfirst_person_character (cast `/Game/FirstPersonBP/Blueprints/FirstPersonCharacter` Pawn))
  (`|AIMoveTo` self (0.0 0.0 0.0) _asfirst_person_character))

(event `self.Box_bullet.OnComponentHit`
  (params (HitComponent :type "PrimitiveComponent Object Reference") (OtherActor :type "Actor Object Reference") (OtherComp :type "PrimitiveComponent Object Reference") (NormalImpulse :type "Vector Structure") (Hit :type "HitResult Structure (by ref)"))
  ;[1 1 1] gets hit by bullet
  (cast `/Game/FirstPersonBP/Blueprints/FirstPersonProjectile` OtherActor)
  (`AudioComponent.Play` (`self.death sound`) 0.0)
  (`KismetSystemLibrary.Delay` 0.2)
  (`self.K2_DestroyActor`))

(event `self.Box_boxmean.OnComponentBeginOverlap`
  (params (OverlappedComponent :type "PrimitiveComponent Object Reference") (OtherActor :type "Actor Object Reference") (OtherComp :type "PrimitiveComponent Object Reference") (OtherBodyIndex :type Integer) (bFromSweep :type Boolean) (SweepResult :type "HitResult Structure (by ref)"))
  ;[1 1 1] gets hit by mean box
  (cast `/Game/MainShit/bps/bp_meanbox` OtherActor)
  (`AudioComponent.Play` (`self.death sound`) 0.0)
  (`KismetSystemLibrary.Delay` 0.2)
  (`self.K2_DestroyActor`))

(event `my ass`
  (bind (_returnvalue_roll _returnvalue_pitch _returnvalue_yaw) (`KismetMathLibrary.BreakRotator` (`KismetMathLibrary.RInterpTo` (`self.K2_GetActorRotation`) (`KismetMathLibrary.FindLookAtRotation` (`self.K2_GetActorLocation`) (`self.K2_GetActorLocation` (`self.player_ref`))) (`GameplayStatics.GetWorldDeltaSeconds`) 50.0)))
  ;[1 1 1] move to player
  (`self.K2_SetActorRotation` (`KismetMathLibrary.MakeRotator` 0.0 0.0 _returnvalue_yaw))
  (`KismetSystemLibrary.Delay` 0.001)
  (`self.my ass`))

(fn `Face Player`)

(fn `UserConstructionScript`)