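; bp_whitty is an actor that keeps turning to face the player character.
; On BeginPlay it caches the player's FirstPersonCharacter, then starts a FacePlayer event that re-calls itself after a very short Delay instead of using Tick.
; Each pass sets only the actor's yaw, interpolated toward the look-at rotation to the player, so it stays upright while tracking.
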(event `self.ReceiveBeginPlay`
  (bind _asfirst_person_character (cast `/Game/FirstPersonBP/Blueprints/FirstPersonCharacter` (`GameplayStatics.GetPlayerCharacter` 0)))
  (set `self.player_ref` _asfirst_person_character)
  (`self.Face Player`))

(event `Face Player`
  (bind (_returnvalue_roll _returnvalue_pitch _returnvalue_yaw) (`KismetMathLibrary.BreakRotator` (`KismetMathLibrary.RInterpTo` (`self.K2_GetActorRotation`) (`KismetMathLibrary.FindLookAtRotation` (`self.K2_GetActorLocation`) (`self.K2_GetActorLocation` (`self.player_ref`))) (`GameplayStatics.GetWorldDeltaSeconds`) 50.0)))
  ;[1 1 1] Face Player
  (`self.K2_SetActorRotation` (`KismetMathLibrary.MakeRotator` 0.0 0.0 _returnvalue_yaw))
  (`KismetSystemLibrary.Delay` 0.001)
  (`self.Face Player`))

(fn `UserConstructionScript`)